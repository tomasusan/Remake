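; BP_FPGTransformActor is an actor that reacts to sphere overlaps and briefly simulates physics on its mesh before reassembling.
; CollisionSphere and TestingSphere forward begin and end overlaps to separate handler functions defined outside this graph, with CollisionSphere also printing the overlapping component's name.
; SetSimulation waits briefly, enables physics on StaticMeshComponent for a short window, then disables it and calls AssembleAllComponent.
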(event OnComponentBeginOverlap(TestingSphere)
  (params (OverlappedComponent :type Primitive%20Component%20Object%20Reference) (OtherActor :type Actor%20Object%20Reference) (OtherComp :type Primitive%20Component%20Object%20Reference) (OtherBodyIndex :type Integer) (bFromSweep :type Boolean) (SweepResult :type Hit%20Result%20Structure%20%28by%20ref%29))
  (Class|FPGTransformActor|SetTestSphereBeginOverlap))

(event OnComponentEndOverlap(TestingSphere)
  (params (OverlappedComponent :type Primitive%20Component%20Object%20Reference) (OtherActor :type Actor%20Object%20Reference) (OtherComp :type Primitive%20Component%20Object%20Reference) (OtherBodyIndex :type Integer))
  (Class|FPGTransformActor|SetTestSphereEndOverlap))

(event OnComponentBeginOverlap(CollisionSphere)
  (params (OverlappedComponent :type Primitive%20Component%20Object%20Reference) (OtherActor :type Actor%20Object%20Reference) (OtherComp :type Primitive%20Component%20Object%20Reference) (OtherBodyIndex :type Integer) (bFromSweep :type Boolean) (SweepResult :type Hit%20Result%20Structure%20%28by%20ref%29))
  (Class|FPGTransformActor|OnBeginOverlap)
  (if (Utilities|IsValid OtherComp)
    (Development|PrintString (Utilities|GetDisplayName OtherComp))))

(event OnComponentEndOverlap(CollisionSphere)
  (params (OverlappedComponent :type Primitive%20Component%20Object%20Reference) (OtherActor :type Actor%20Object%20Reference) (OtherComp :type Primitive%20Component%20Object%20Reference) (OtherBodyIndex :type Integer))
  (Class|FPGTransformActor|OnEndOverlap))

(event EventBeginPlay)

(event Collision|EventActorBeginOverlap
  (params (OtherActor :type Actor%20Object%20Reference)))

(event EventTick
  (params (DeltaSeconds :type Float%20%28single-precision%29)))

(event EventSetSimulation
  (bind _staticmeshcomponent (Variables|Default|GetStaticMeshComponent))
  (Utilities|FlowControl|Delay 0.5)
  (Physics|SetSimulatePhysics _staticmeshcomponent true)
  (Utilities|FlowControl|Delay 1.0)
  (Physics|SetSimulatePhysics _staticmeshcomponent false)
  (Class|FPGTransformActor|AssembleAllComponent))

(fn ConstructionScript)