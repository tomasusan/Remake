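; Base Blueprint for pickable item actors, providing a world-space "detected" indicator through a widget component.
; BeginPlay caches the component's WBP_DetectedWidget, and the fade-in and fade-out events forward to that widget's FadeIn and FadeOut.
; Tick rotates the widget component every frame to face the player camera manager, acting as a billboard.
; The file itself contains no pickup or detection logic.
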(event EventBeginPlay
  (bind _aswbp_detected_widget (Utilities|Casting|CastToWBP_DetectedWidget (UserInterface|GetWidget (Variables|Default|GetDetectedWidget))))
  (Variables|Default|SetDetectedWidgetPtr _aswbp_detected_widget))

(event Collision|EventActorBeginOverlap
  (params (OtherActor :type Actor%20Object%20Reference)))

(event EventTick
  (params (DeltaSeconds :type Float%20%28single-precision%29))
  (bind _detectedwidget (Variables|Default|GetDetectedWidget))
  (Transformation|SetWorldRotation _detectedwidget (Math|Rotator|FindLookatRotation (Transformation|GetWorldLocation _detectedwidget) (Transformation|GetActorLocation (Game|GetPlayerCameraManager 0))) false false))

(event EventPlayAnimationFadein
  (Default|Fadein (Variables|Default|GetDetectedWidgetPtr)))

(event EventPlayAnimationFadeout
  (Default|FadeOut (Variables|Default|GetDetectedWidgetPtr)))

(fn ConstructionScript)